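; BP_JoinTrigger is a Mordhau box trigger that collects the characters standing inside it for a later group teleport.
; Overlap begin and end events add and remove characters in PlayersToTeleport, gated by a game mode cast that confines tracking to the server.
; MoveToTop teleports each tracked character to a random spot around the world origin at a fixed height and zeroes its received fall damage, with debug prints throughout.
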(event OnComponentBeginOverlap(Box)
  (params (OverlappedComponent :type Primitive%20Component%20Object%20Reference) (OtherActor :type Actor%20Object%20Reference) (OtherComp :type Primitive%20Component%20Object%20Reference) (OtherBodyIndex :type Integer) (bFromSweep :type Boolean) (SweepResult :type Hit%20Result%20Structure%20%28by%20ref%29))
  (bind _playerstoteleport (Variables|Default|GetPlayersToTeleport))
  (Utilities|Casting|CastToBP_MordhauGameMode (Game|GetGameMode))
  (bind _asbp_mordhau_character (Utilities|Casting|CastToBP_MordhauCharacter OtherActor))
  (Utilities|Array|AddUnique _playerstoteleport _asbp_mordhau_character)
  (Development|PrintString "SOMEONE WENT IN")
  (Development|PrintString (Utilities|String|ToString(Integer) (Utilities|Array|Length _playerstoteleport))))

(event OnComponentEndOverlap(Box)
  (params (OverlappedComponent :type Primitive%20Component%20Object%20Reference) (OtherActor :type Actor%20Object%20Reference) (OtherComp :type Primitive%20Component%20Object%20Reference) (OtherBodyIndex :type Integer))
  (Utilities|Casting|CastToBP_MordhauGameMode (Game|GetGameMode))
  (bind _asbp_mordhau_character (Utilities|Casting|CastToBP_MordhauCharacter OtherActor))
  (Utilities|Array|RemoveItem (Variables|Default|GetPlayersToTeleport) _asbp_mordhau_character)
  (Development|PrintString "SOMEONE WENT OUT"))

(event Custom|MoveToTop
  (for _array_element (Variables|Default|GetPlayersToTeleport)
    (bind _asbp_mordhau_character (Utilities|Casting|CastToBP_MordhauCharacter _array_element))
    (bind _returnvalue (Transformation|Teleport _asbp_mordhau_character (Math|Vector|MakeVector (Math|Conversions|ToFloat(Integer) (Math|Random|RandomIntegerinRange -500 500)) (Math|Conversions|ToFloat(Integer) (Math|Random|RandomIntegerinRange -500 500)) 3e+02) "0, 0, 0"))
    (Variables|/Script/Mordhau.AdvancedCharacter|SetReceivedFallDamageModifier _asbp_mordhau_character 0.0)
    (Development|PrintString (Utilities|String|ToString(Boolean) _returnvalue) true true "(R=0.096780,G=1.000000,B=0.000000,A=1.000000)" 1e+01)))

(event EventBeginPlay
  (|CallParentFunction) ; This node is disabled and will not be called.\nDrag off pins to build functionality.
)

(event EventTick
  (params (DeltaSeconds :type Float%20%28single-precision%29))
  (|CallParentFunction DeltaSeconds) ; This node is disabled and will not be called.\nDrag off pins to build functionality.
)

(fn ConstructionScript
  (|CallParentFunction))