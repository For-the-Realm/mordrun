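; BP_Platform2 is a one-shot breakable platform that destroys itself shortly after something overlaps its Box trigger.
; The first overlap, gated by a game mode cast that limits logic to the server, turns it purple, waits, flags it dead, then destroys it after a brief delay.
; RepNotify variables apply the material to the Cube and R components and play the barrel-breaking sound.
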(event OnComponentBeginOverlap(Box)
  (params (OverlappedComponent :type Primitive%20Component%20Object%20Reference) (OtherActor :type Actor%20Object%20Reference) (OtherComp :type Primitive%20Component%20Object%20Reference) (OtherBodyIndex :type Integer) (bFromSweep :type Boolean) (SweepResult :type Hit%20Result%20Structure%20%28by%20ref%29))
  (Utilities|FlowControl|DoOnce false
    (:Completed
      (Utilities|Casting|CastToMordhauGameMode (Game|GetGameMode))
      (Variables|Default|SetPlatformMaterial "/MordRun/M_MR_Purple.M_MR_Purple")
      (Utilities|FlowControl|Delay 3.0)
      (Variables|Default|SetDead true)
      (Utilities|FlowControl|Delay 0.5)
      (Actor|DestroyActor))))

(event EventBeginPlay
  (|CallParentFunction) ; This node is disabled and will not be called.\nDrag off pins to build functionality.
)

(event Collision|EventActorBeginOverlap
  (params (OtherActor :type Actor%20Object%20Reference))
  (|CallParentFunction OtherActor) ; This node is disabled and will not be called.\nDrag off pins to build functionality.
)

(event EventTick
  (params (DeltaSeconds :type Float%20%28single-precision%29))
  (|CallParentFunction DeltaSeconds) ; This node is disabled and will not be called.\nDrag off pins to build functionality.
)

(fn ConstructionScript
  (|CallParentFunction))

(fn OnRepPlatformMaterial
  (bind _platformmaterial (Variables|Default|GetPlatformMaterial))
  (Rendering|Material|SetMaterial (Variables|Default|GetCube) 0 _platformmaterial)
  (Rendering|Material|SetMaterial (Variables|Default|Getr) 0 _platformmaterial))

(fn OnRepDead
  (Audio|SpawnSoundatLocation "/Game/Mordhau/Audio/Cues/Siege/SC_BarrelBreaking.SC_BarrelBreaking" (Transformation|GetWorldLocation (Variables|Default|GetCube)) "0, 0, 0" 0.5 1.0 0.0 0 0))