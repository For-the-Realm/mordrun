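; Match controller for the MordRun mode in Mordhau, cycling between Waiting and Running phases on Tick-driven countdowns.
; Each match start enables the floor, rebuilds stacked grids of BP_Platform2, teleports players from BP_JoinTrigger above them without fall damage, and broadcasts a warning.
; After a 10-second delay the floor is hidden and loses collision.
; Timer text updates every tick on BP_MatchDetails actors, while the MatchStatus RepNotify sets their status text.
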(event Custom|MovePlayersToTopEvent
  (bind _outactors (Actor|GetAllActorsOfClass "/MordRun/BPs/BP_JoinTrigger.BP_JoinTrigger_C"))
  (for _array_element _outactors
    (bind _output_get (Variables|Default|SetPlayersToTeleportBackup (Variables|/MordRun/BPs/BP_JoinTrigger.BP_JoinTrigger_C|GetPlayersToTeleport _array_element)))
    (for _array_element_2 _output_get
      (Development|PrintString "shit" true true "(R=0.000000,G=0.660000,B=1.000000,A=1.000000)" 1e+01)
      (bind _asbp_mordhau_character (Utilities|Casting|CastToBP_MordhauCharacter _array_element_2))
      (bind _returnvalue (Transformation|Teleport _asbp_mordhau_character (Math|Vector|MakeVector (Math|Conversions|ToFloat(Integer) (Math|Random|RandomIntegerinRange -500 500)) (Math|Conversions|ToFloat(Integer) (Math|Random|RandomIntegerinRange -500 500)) 3e+02) "0, 0, 0"))
      (Variables|/Script/Mordhau.AdvancedCharacter|SetReceivedFallDamageModifier _asbp_mordhau_character 0.0)
      (Development|PrintString (Utilities|String|ToString(Boolean) _returnvalue) true true "(R=0.096780,G=1.000000,B=0.000000,A=1.000000)" 1e+01))))

(event Custom|BeginMordRun
  (CallFunction|EnableFloor)
  (CallFunction|RecreatePlatforms)
  (Utilities|FlowControl|Delay 1e+01)
  (CallFunction|DisableFloor))

(event EventBeginPlay
  (|CallParentFunction))

(event Collision|EventActorBeginOverlap
  (params (OtherActor :type Actor%20Object%20Reference))
  (|CallParentFunction OtherActor) ; This node is disabled and will not be called.\nDrag off pins to build functionality.
)

(event EventTick
  (params (DeltaSeconds :type Float%20%28single-precision%29))
  (bind _defaultwaittime (Variables|Default|GetDefaultWaitTime))
  (bind _defaultmatchtime (Variables|Default|GetDefaultMatchTime))
  (|CallParentFunction DeltaSeconds)
  (CallFunction|UpdateTimers)
  (if (Utilities|Enum|Equal(Enum) (Variables|Default|GetMatchStatus) "Running")
    (bind _output_get (Variables|Default|SetMatchTimer (- (Variables|Default|GetMatchTimer) DeltaSeconds)))
    ;[1 1 1] Match is now over
    (if (< _output_get 0.0)
      (Variables|Default|SetMatchStatus "Waiting")
      (Variables|Default|SetMatchTimer _defaultmatchtime)
      (Variables|Default|SetWaitTimer _defaultwaittime))
    (elif (Utilities|Enum|Equal(Enum) (Variables|Default|GetMatchStatus) "Waiting")
      (bind _output_get_2 (Variables|Default|SetWaitTimer (- (Variables|Default|GetWaitTimer) DeltaSeconds)))
      ;[1 1 1] Waiting is over
      (if (< _output_get_2 0.0)
        (Variables|Default|SetMatchStatus "Running")
        (Variables|Default|SetMatchTimer _defaultmatchtime)
        (Variables|Default|SetWaitTimer _defaultwaittime)
        (CallFunction|BeginMordRun)
        (CallFunction|MovePlayerstoTopEvent)
        (bind _asbp_mordhau_game_mode (Utilities|Casting|CastToBP_MordhauGameMode (Game|GetGameMode)))
        (Class|MordhauGameMode|Broadcast _asbp_mordhau_game_mode self "Get ready! Match will begin in 10 seconds." "ServerSay")))))

(fn ConstructionScript
  (|CallParentFunction))

(fn DisableFloor
  (Utilities|Casting|CastToBP_MordhauGameMode (Game|GetGameMode))
  ;[1 1 1] Disable Floor + Block movement zone
  (bind _outactors (Actor|GetAllActorsOfClass "/MordRun/BPs/BP_Floor.BP_Floor_C"))
  (for _array_element _outactors
    (Rendering|SetActorHiddenInGame _array_element true)
    (Collision|SetActorEnableCollision _array_element false)))

(fn RecreatePlatforms
  (bind _asbp_mordhau_game_mode (Utilities|Casting|CastToBP_MordhauGameMode (Game|GetGameMode)))
  ;[1 1 1] Recreate Platforms
  (bind _outactors (Class|MordhauUtilityLibrary|GetAllActorsinLevelOfClass _asbp_mordhau_game_mode "/MordRun/BPs/BP_Platform2.BP_Platform2_C" "FFA_MordRun_LevelOne"))
  (for _array_element _outactors
    (Actor|DestroyActor _array_element))
  (for _index (range 0 3)
    (CallFunction|CreateLevel _index 20 20)))

(fn EnableFloor
  (Utilities|Casting|CastToBP_MordhauGameMode (Game|GetGameMode))
  ;[1 1 1] Re-enable Floor + Block movement zone
  (bind _outactors (Actor|GetAllActorsOfClass "/MordRun/BPs/BP_Floor.BP_Floor_C"))
  (for _array_element _outactors
    (Rendering|SetActorHiddenInGame _array_element false)
    (Collision|SetActorEnableCollision _array_element true)))

(fn ClearPlayerstoTeleport)

(fn UpdateTimers
  (bind _asmordhau_game_mode (Utilities|Casting|CastToMordhauGameMode (Game|GetGameMode)))
  (bind _outactors (Class|MordhauUtilityLibrary|GetAllActorsinLevelOfClass _asmordhau_game_mode "/MordRun/BPs/BP_MatchDetails.BP_MatchDetails_C" (Class|MordhauUtilityLibrary|GetActorLevelName _asmordhau_game_mode)))
  (for _array_element _outactors
    (if (Utilities|Enum|Equal(Enum) (Variables|Default|GetMatchStatus) "Running")
      (Variables|/MordRun/BPs/BP_MatchDetails.BP_MatchDetails_C|SetTimerText _array_element (Utilities|String|Append (Utilities|String|ToString(Integer) (Math|Float|Floor (Variables|Default|GetMatchTimer))) "s"))
      (elif (Utilities|Enum|Equal(Enum) (Variables|Default|GetMatchStatus) "Waiting")
        (Variables|/MordRun/BPs/BP_MatchDetails.BP_MatchDetails_C|SetTimerText _array_element (Utilities|String|Append (Utilities|String|ToString(Integer) (Math|Float|Floor (Variables|Default|GetWaitTimer))) "s"))))))

(fn CreateLevel
  (params (Level :type Integer) (Width :type Integer) (Height :type Integer))
  (bind _distancebetweenplatforms (Variables|Default|GetDistanceBetweenPlatforms))
  ;[1 1 1] Function: Create Level - Creates a grid of platforms at Level, which contain Width * Depth platforms
  (for _index (range 0 Height)
    (for _index_2 (range 0 Width)
      (Game|SpawnActorfromClass "/MordRun/BPs/BP_Platform2.BP_Platform2_C" (Math|Transform|MakeTransform (Math|Vector|MakeVector (Math|Conversions|ToFloat(Integer) (- (Variables|Default|GetOffsetX) (* _distancebetweenplatforms _index))) (Math|Conversions|ToFloat(Integer) (- (Variables|Default|GetOffsetY) (* _index_2 _distancebetweenplatforms))) (Math|Conversions|ToFloat(Integer) (- (Variables|Default|GetStartingZ) (* Level (Variables|Default|GetDistanceBetweenLevels)))))) "Undefined" 0 0))))

(fn OnRepMatchStatus
  (bind _asbp_mordhau_game_mode (Utilities|Casting|CastToBP_MordhauGameMode (Game|GetGameMode)))
  (bind _returnvalue (Game|GetCurrentLevelName true))
  (bind _outactors (Class|MordhauUtilityLibrary|GetAllActorsinLevelOfClass _asbp_mordhau_game_mode "/MordRun/BPs/BP_MatchDetails.BP_MatchDetails_C" _returnvalue))
  (for _array_element _outactors
    (if (Utilities|Enum|Equal(Enum) (Variables|Default|GetMatchStatus) "Running")
      (Variables|/MordRun/BPs/BP_MatchDetails.BP_MatchDetails_C|SetStatusText _array_element (Utilities|String|ToString(Text) (Utilities|Text|ToText(String) "Match in progress.")))
      (elif (Utilities|Enum|Equal(Enum) (Variables|Default|GetMatchStatus) "Waiting")
        (Variables|/MordRun/BPs/BP_MatchDetails.BP_MatchDetails_C|SetStatusText _array_element (Utilities|String|ToString(Text) (Utilities|Text|ToText(String) "Starting match. Wait here to join.")))))))